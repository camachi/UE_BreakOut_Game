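; BP_Block is a destructible brick actor that takes a set number of hits before it is destroyed.
; Each Hit event decrements HitsToDestroy, refreshes the color, prints a debug string and destroys the actor once the count reaches zero.
; ChangeColor, also run at BeginPlay, switches on the remaining hits to apply a red, yellow or green material instance to the mesh.
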(event Collision|EventActorBeginOverlap
  (params (OtherActor :type Actor%20Object%20Reference)))

(event EventTick
  (params (DeltaSeconds :type Float%20%28single-precision%29)))

(event Collision|EventHit
  (params (MyComp :type Primitive%20Component%20Object%20Reference) (Other :type Actor%20Object%20Reference) (OtherComp :type Primitive%20Component%20Object%20Reference) (bSelfMoved :type Boolean) (HitLocation :type Vector :default "0, 0, 0") (HitNormal :type Vector :default "0, 0, 0") (NormalImpulse :type Vector :default "0, 0, 0") (Hit :type Hit%20Result%20Structure%20%28by%20ref%29))
  (bind _output_get (Variables|Default|SetHitsToDestroy (- (Variables|Default|GetHitsToDestroy) 1)))
  (CallFunction|ChangeColor)
  (Development|PrintString "hit")
  (if (<= _output_get 0)
    (Actor|DestroyActor)))

(event EventBeginPlay
  (CallFunction|ChangeColor))

(fn ConstructionScript)

(fn ChangeColor
  (switch int (Variables|Default|GetHitsToDestroy)
    (:1
      (bind _output_get (Variables|Default|SetNewColorMat "/Game/Materials/MI_BrickColorRed.MI_BrickColorRed"))
      (Rendering|Material|SetMaterial (Variables|Default|GetStaticMesh) 0 _output_get))
    (:2
      (bind _output_get_2 (Variables|Default|SetNewColorMat "/Game/Materials/MI_BrickColorYellow.MI_BrickColorYellow"))
      (Rendering|Material|SetMaterial (Variables|Default|GetStaticMesh) 0 _output_get_2))
    (:3
      (bind _output_get_3 (Variables|Default|SetNewColorMat "/Game/Materials/MI_BrickColorGreen.MI_BrickColorGreen"))
      (Rendering|Material|SetMaterial (Variables|Default|GetStaticMesh) 0 _output_get_3))))