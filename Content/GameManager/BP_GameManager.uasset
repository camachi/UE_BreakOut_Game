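; BP_GameManager starts the match with a countdown and then puts the ball into play.
; On BeginPlay it creates the WBP_CountDown widget, adds it to the viewport, binds SpawnBall to its countdown-finished event and starts the countdown.
; SpawnBall spawns an actor of BallClass at the transform of the BallSpawner actor.
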(event Custom|SpawnBall
  (Game|SpawnActorfromClass (Variables|Default|GetBallClass) (Transformation|GetActorTransform (Variables|Default|GetBallSpawner)) "Undefined" "MultiplyWithRoot" 0 0))

(event EventBeginPlay
  (bind _returnvalue (UserInterface|CreateWidget "/Game/UserInterface/WBP_CountDown.WBP_CountDown_C"))
  (bind _output_get (Variables|Default|SetCountdownwidgetref _returnvalue))
  (UserInterface|Viewport|AddtoViewport _output_get 0)
  (EventDispatchers|BindEventtoOnCountdownFinished (Variables|Default|GetCountdownwidgetref) (delegate Custom|SpawnBall))
  (Default|StartCountdown (Variables|Default|GetCountdownwidgetref)))

(fn ConstructionScript)