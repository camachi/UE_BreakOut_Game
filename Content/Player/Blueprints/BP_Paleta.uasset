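; BP_Paleta is a player-controlled paddle actor that slides side to side along the world Y axis.
; On BeginPlay it enables input from player controller 0, then the MoveRight axis event offsets its location by the axis value times PlayerVelocity.
; Y is clamped to a fixed symmetric range while X and Z stay unchanged.
; Movement sets the location directly without sweep and is not scaled by delta time.
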(event EventBeginPlay
  (Input|EnableInput (Game|GetPlayerController 0)))

(event Collision|EventActorBeginOverlap
  (params (OtherActor :type Actor%20Object%20Reference)))

(event EventTick
  (params (DeltaSeconds :type Float%20%28single-precision%29)))

(event Input|AxisEvents|InputAxisMoveRight
  (params (AxisValue :type Float%20%28single-precision%29))
  (bind _returnvalue (Transformation|GetActorLocation))
  (bind (_x _y _z) (Math|Vector|BreakVector _returnvalue))
  (Transformation|SetActorLocation (Math|Vector|MakeVector _x (Math|Float|Clamp(Float) (+ _y (* AxisValue (Variables|Default|GetPlayerVelocity))) -6e+02 6e+02) _z) false false))

(fn ConstructionScript)